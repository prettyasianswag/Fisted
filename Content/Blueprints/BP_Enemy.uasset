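; Enemy character Blueprint that chases the player, punches on arrival and reloads Map_Prototype when its punch sphere overlaps BP_FighterCharacter.
; Tick drives gated AIMoveTo; success sets the AnimBlueprint's CanPunch and closes the gate until ChasePlayerAgain reopens it.
; Separate events toggle the punch sphere's collision.
; EnemyDefeated applies damage with a short re-hit lockout, switching to physics with a knockback impulse when health runs out.
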(event `ActivatePunchCollider`
  (bind _sphere (`self.Sphere`))
  ;[1 1 1] ActivatePunchCollider
  (`PrimitiveComponent.SetCollisionEnabled` _sphere "QueryOnly")
  (`PrimitiveComponent.SetCollisionResponseToAllChannels` _sphere "ECR_Overlap"))

(event `DeactivatePunchCollider`
  ;[1 1 1] DeactivatePunchCollider
  (`PrimitiveComponent.SetCollisionEnabled` (`self.Sphere`) "NoCollision"))

(event `self.ReceiveTick`
  (params (DeltaSeconds :type "Float (single-precision)"))
  ;[1 1 1] EventTick
  ;;[1 1 1] MoveToThePlayer
  (`/Engine/EditorBlueprintResources/StandardMacros.Gate` false :!label _label
    (:`Exit`
      (`|AIMoveTo` self (0.0 0.0 0.0) (`GameplayStatics.GetPlayerCharacter` 0) 120.0
        (:`OnSuccess`
          (`|ExecutionSequence`
            (:`then_0`
              ;;[1 1 1] OnlyPunchOncePerSecond
              (`/Engine/EditorBlueprintResources/StandardMacros.DoOnce` false :!label _label_2
                (:`Completed`
                  ;;[1 1 1] PunchPlayerAnimation
                  (bind _asue4asp_hero_tpp_anim_blueprint (cast `/Game/AnimStarterPack/UE4ASP_HeroTPP_AnimBlueprint` (`SkeletalMeshComponent.GetAnimInstance` (`self.Mesh`))))
                  (set `/Game/AnimStarterPack/UE4ASP_HeroTPP_AnimBlueprint.CanPunch` true _asue4asp_hero_tpp_anim_blueprint)
                  (goto _label_2 :!via `Reset`))))
            (:`then_1`
              (goto _label :!via `Close`))))))))

(event `ChasePlayerAgain`
  ;[1 1 1] EventTick
  (goto _label :!via `Open`))

(event `self.Sphere.OnComponentBeginOverlap`
  (params (OverlappedComponent :type "PrimitiveComponent Object Reference") (OtherActor :type "Actor Object Reference") (OtherComp :type "PrimitiveComponent Object Reference") (OtherBodyIndex :type Integer) (bFromSweep :type Boolean) (SweepResult :type "HitResult Structure (by ref)"))
  (cast `/Game/Blueprints/BP_FighterCharacter` OtherActor)
  (`GameplayStatics.OpenLevel` "Map_Prototype"))

(event `EnemyDefeated`
  (params (Damage :type Integer) (KnockBackDirection :type "Vector Structure"))
  (bind (_returnvalue_x _returnvalue_y) (`KismetMathLibrary.BreakVector` (* KnockBackDirection (`self.KnockbackAmount`))))
  ;[1 1 1] EnemyDefeated
  (`/Engine/EditorBlueprintResources/StandardMacros.DoOnce` false :!label _label_3
    (:`Completed`
      (set `self.Health` (- (`self.Health`) Damage))
      (`|ExecutionSequence`
        (:`then_0`
          (if (<= (`self.Health`) 0)
            (`/Engine/EditorBlueprintResources/StandardMacros.DoOnce` false
              (:`Completed`
                (`PrimitiveComponent.SetSimulatePhysics` (`self.Mesh`) true)
                (`PrimitiveComponent.SetCollisionEnabled` (`self.CapsuleComponent`) "NoCollision")
                (`PrimitiveComponent.AddImpulse` (`self.Mesh`) (`KismetMathLibrary.MakeVector` _returnvalue_x _returnvalue_y 50000.0) "None" false)))))
        (:`then_1`
          (`KismetSystemLibrary.Delay` 0.4)
          (goto _label_3 :!via `Reset`))))))

(fn `UserConstructionScript`)